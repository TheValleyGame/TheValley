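; A moving platform that lights up while the IcaroBP actor is inside its Box volume.
; On BeginPlay a timeline drives the static mesh along the actor's forward vector, adding the scaled Offset to its current location each update, so movement accumulates rather than following the stored start position.
; The construction script gives the mesh a dynamic material instance, whose "Brillo" parameter the overlap events raise and reset.
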(event `self.ReceiveBeginPlay`
  (set `self.iniPos` (`self.K2_GetActorLocation`))
  (bind (_direction _offset) (`Timeline|Timeline_0` :!via `PlayFromStart`)
    (:`Update`
      (`SceneComponent.K2_SetWorldLocation` (`self.StaticMesh`) (+ (* (`self.GetActorForwardVector`) (* (`self.Offset`) _offset)) (`SceneComponent.K2_GetComponentLocation` (`self.StaticMesh`))) false false))))

(event `self.Box.OnComponentBeginOverlap`
  (params (OverlappedComponent :type "PrimitiveComponent Object Reference") (OtherActor :type "Actor Object Reference") (OtherComp :type "PrimitiveComponent Object Reference") (OtherBodyIndex :type Integer) (bFromSweep :type Boolean) (SweepResult :type "HitResult Structure (by ref)"))
  (cast `/Game/Blueprints/IcaroBP` OtherActor)
  (`MaterialInstanceDynamic.SetScalarParameterValue` (`self.platformMaterial`) "Brillo" 5.0))

(event `self.Box.OnComponentEndOverlap`
  (params (OverlappedComponent :type "PrimitiveComponent Object Reference") (OtherActor :type "Actor Object Reference") (OtherComp :type "PrimitiveComponent Object Reference") (OtherBodyIndex :type Integer))
  (cast `/Game/Blueprints/IcaroBP` OtherActor)
  (`MaterialInstanceDynamic.SetScalarParameterValue` (`self.platformMaterial`) "Brillo" 0.0))

(fn `UserConstructionScript`
  (bind _returnvalue (`KismetMaterialLibrary.CreateDynamicMaterialInstance` "/Game/Blueprints/Materials/PlatformMaterial_Inst.PlatformMaterial_Inst"))
  (bind _output_get (set `self.platformMaterial` _returnvalue))
  (`PrimitiveComponent.SetMaterial` (`self.StaticMesh`) 0 _output_get))