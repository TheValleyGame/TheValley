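; Automated cannon turret that aims toward player 0's pawn and fires projectiles.
; Tick applies constant-rate look-at interpolation to base yaw and barrel yaw and pitch; yaw steps from the actor's rotation each frame, so it stays near that heading.
; From BeginPlay, ShootEvt re-calls itself after short random delays, spawning a half-scale ProyectileMesh at ShootLocation with an impulse and slightly randomized forward direction.
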(event `self.ReceiveBeginPlay`
  (`self.ShootEvt`))

(event `ShootEvt`
  (bind _canionsm (`self.CanionSM`))
  (`KismetSystemLibrary.Delay` (`KismetMathLibrary.RandomFloatInRange` 0.1 2.0))
  (`|SpawnActorFromClass` "/Game/Blueprints/Game/proyectileMesh.proyectileMesh_C" (`KismetMathLibrary.MakeTransform` (`SceneComponent.K2_GetComponentLocation` (`self.ShootLocation`)) (`SceneComponent.K2_GetComponentRotation` _canionsm) (0.5 0.5 0.5)) "AlwaysSpawn" "OverrideRootScale" null (+ (`SceneComponent.GetForwardVector` _canionsm) (* (`KismetMathLibrary.RandomUnitVector`) 0.1)) 4000.0 null)
  (`self.ShootEvt`))

(event `self.ReceiveTick`
  (params (DeltaSeconds :type "Float (single-precision)"))
  (bind _returnvalue (`KismetMathLibrary.FInterpTo_Constant` (.yaw (`self.K2_GetActorRotation`)) (.yaw (`KismetMathLibrary.FindLookAtRotation` (`SceneComponent.K2_GetComponentLocation` (`self.CanionSM`)) (`self.K2_GetActorLocation` (`GameplayStatics.GetPlayerPawn` 0)))) DeltaSeconds 40.0))
  (`SceneComponent.K2_SetWorldRotation` (`self.BaseSM`) (`KismetMathLibrary.MakeRotator` 0.0 0.0 _returnvalue) false false)
  (`SceneComponent.K2_SetWorldRotation` (`self.CanionSM`) (`KismetMathLibrary.MakeRotator` 0.0 (`KismetMathLibrary.FInterpTo_Constant` (.pitch (`SceneComponent.K2_GetComponentRotation` (`self.CanionSM`))) (.pitch (`KismetMathLibrary.FindLookAtRotation` (`SceneComponent.K2_GetComponentLocation` (`self.CanionSM`)) (`self.K2_GetActorLocation` (`GameplayStatics.GetPlayerPawn` 0)))) (`GameplayStatics.GetWorldDeltaSeconds`) 40.0) _returnvalue) false false))

(fn `UserConstructionScript`)