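; Game instance Blueprint that tracks the player's key count in an SInventory struct.
; AddKeys increases NumKeys, and ConsumeKeys subtracts from it and returns a success flag.
; The sufficient-keys comparison in ConsumeKeys is left unconnected, so its branch always succeeds and the count can go negative.
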(fn `AddKeys`
  (params (numKeys :type Integer))
  (setmembers `/Game/Blueprints/Game/sInventory` :`StructRef` (`self.sInventory`) :`numKeys` (+ numKeys (`.numKeys_2_103C92324F3D5BAF7043709E73F4C182` (break `/Game/Blueprints/Game/sInventory` (`self.sInventory`)))))
  (return))

(fn `ConsumeKeys`
  (params (numKeys :type Integer))
  (returns (Succes :type Boolean))
  (if true
    (setmembers `/Game/Blueprints/Game/sInventory` :`StructRef` (`self.sInventory`) :`numKeys` (- (`.numKeys_2_103C92324F3D5BAF7043709E73F4C182` (break `/Game/Blueprints/Game/sInventory` (`self.sInventory`))) numKeys))
    (return true)
    (else
      (return false))))