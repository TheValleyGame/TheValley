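; Moving platform Blueprint that shifts its PlatformSM component along the actor's forward axis once play begins.
; BeginPlay starts the MOVEMENT timeline, whose Offset track scales the Offset variable on each update.
; Each step adds to the component's current world location without sweeping, so movement accumulates per update, and the stored start location IniPos goes unused here.
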(event `self.ReceiveBeginPlay`
  (set `self.iniPos` (`self.K2_GetActorLocation`))
  (bind (_direction _offset) (`Timeline|MOVEMENT` :!via `PlayFromStart`)
    (:`Update`
      (`SceneComponent.K2_SetWorldLocation` (`self.PlatformSM`) (+ (* (`self.GetActorForwardVector`) (* (`self.Offset`) _offset)) (`SceneComponent.K2_GetComponentLocation` (`self.PlatformSM`))) false false))))

(fn `UserConstructionScript`)