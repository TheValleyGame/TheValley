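; Key-locked sliding door that opens for the ThirdPersonCharacter in exchange for a set number of keys.
; Entering the Box asks the game instance to consume NumKeys; on success a timeline moves the door mesh along relative Z, and leaving reverses it.
; A separate console collider shows the key cost as two-digit text while overlapped.
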(event `self.Box.OnComponentBeginOverlap`
  (params (OverlappedComponent :type "PrimitiveComponent Object Reference") (OtherActor :type "Actor Object Reference") (OtherComp :type "PrimitiveComponent Object Reference") (OtherBodyIndex :type Integer) (bFromSweep :type Boolean) (SweepResult :type "HitResult Structure (by ref)"))
  (cast `/Game/ThirdPersonBP/Blueprints/ThirdPersonCharacter` OtherActor)
  (bind _succes (`/Game/Blueprints/Game/mygameinstance.ConsumeKeys` (cast `/Game/Blueprints/Game/mygameinstance` (`GameplayStatics.GetGameInstance`) :!pure true) (`self.numKeys`)))
  (if _succes
    (bind (_direction _newtrack_1) (`Timeline|SlidingDoor TL` :!label _label)
      (:`Update`
        (`SceneComponent.K2_SetRelativeLocation` (`self.DoorSM`) (`KismetMathLibrary.MakeVector` 0.0 0.0 _newtrack_1) false false)))))

(event `self.Box.OnComponentEndOverlap`
  (params (OverlappedComponent :type "PrimitiveComponent Object Reference") (OtherActor :type "Actor Object Reference") (OtherComp :type "PrimitiveComponent Object Reference") (OtherBodyIndex :type Integer))
  (cast `/Game/ThirdPersonBP/Blueprints/ThirdPersonCharacter` OtherActor)
  (goto _label :!via `Reverse`))

(event `self.ConsoleCollider.OnComponentBeginOverlap`
  (params (OverlappedComponent :type "PrimitiveComponent Object Reference") (OtherActor :type "Actor Object Reference") (OtherComp :type "PrimitiveComponent Object Reference") (OtherBodyIndex :type Integer) (bFromSweep :type Boolean) (SweepResult :type "HitResult Structure (by ref)"))
  (cast `/Game/ThirdPersonBP/Blueprints/ThirdPersonCharacter` OtherActor)
  (`TextRenderComponent.K2_SetText` (`self.TextRender`) (`KismetTextLibrary.Conv_IntToText` (`self.numKeys`) true 2 2))
  (`SceneComponent.SetVisibility` (`self.TextRender`) true false))

(event `self.ConsoleCollider.OnComponentEndOverlap`
  (params (OverlappedComponent :type "PrimitiveComponent Object Reference") (OtherActor :type "Actor Object Reference") (OtherComp :type "PrimitiveComponent Object Reference") (OtherBodyIndex :type Integer))
  (`SceneComponent.SetVisibility` (`self.TextRender`) false false))

(fn `UserConstructionScript`)