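; PlatformBP is a moving platform whose static mesh oscillates back and forth along the world X or Y axis.
; BeginPlay stores the mesh's starting world location as the center of the motion.
; Each Tick offsets it by a sine of game time, scaled by Period and amplitude Recorrido, on the axis chosen by SentidoMovimiento.
; The location is set directly without sweep, using 6.3 as an approximate 2π.
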(event `self.ReceiveBeginPlay`
  (set `self.initialLocation` (`SceneComponent.K2_GetComponentLocation` (`self.StaticMesh`))))

(event `self.ReceiveTick`
  (params (DeltaSeconds :type "Float (single-precision)"))
  (bind _initiallocation (`self.initialLocation`))
  (bind _staticmesh (`self.StaticMesh`))
  (bind _returnvalue (* (`KismetMathLibrary.Sin` (/ (* (`KismetSystemLibrary.GetGameTimeInSeconds`) 6.3) (`self.period`))) (`self.recorrido`)))
  (switch `/Game/Blueprints/EsentidoPlataforma` (`self.SentidoMovimiento`)
    (:`NewEnumerator0`
      (`SceneComponent.K2_SetWorldLocation` _staticmesh (+ _initiallocation (`KismetMathLibrary.MakeVector` _returnvalue)) false false))
    (:`NewEnumerator1`
      (`SceneComponent.K2_SetWorldLocation` _staticmesh (+ _initiallocation (`KismetMathLibrary.MakeVector` 0.0 _returnvalue)) false false))))

(fn `UserConstructionScript`)